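; BP_Dummy is a target character that the player can stealth-assassinate from behind.
; A sphere overlap with BP_ThirdPersonCharacter toggles the AssasinateWidget prompt, which Tick re-orients using the camera's forward vector as a look-at point.
; StealthBackAssassination plays the victim knife montage, hides the prompt, triggers a delayed ragdoll and returns a reference location and actor rotation.
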(event `self.ReceiveTick`
  (params (DeltaSeconds :type "Float (single-precision)"))
  ;[1 1 1] Set Widget Rotation
  (`SceneComponent.K2_SetWorldRotation` (`self.AssasinateWidget`) (`KismetMathLibrary.FindLookAtRotation` (`SceneComponent.K2_GetComponentLocation` (`self.AssasinateWidget`)) (`KismetMathLibrary.Conv_RotatorToVector` (`SceneComponent.K2_GetComponentRotation` (`PlayerCameraManager.TransformComponent` (`GameplayStatics.GetPlayerCameraManager` 0))))) false false))

(event `Ragdoll`
  ;[1 1 1] Ragdoll Physics Sumation
  (`KismetSystemLibrary.Delay` 2.5)
  (`PrimitiveComponent.SetSimulatePhysics` (`self.Mesh`) true))

(event `self.AssassinationSph.OnComponentBeginOverlap`
  (params (OverlappedComponent :type "PrimitiveComponent Object Reference") (OtherActor :type "Actor Object Reference") (OtherComp :type "PrimitiveComponent Object Reference") (OtherBodyIndex :type Integer) (bFromSweep :type Boolean) (SweepResult :type "HitResult Structure (by ref)"))
  ;[1 1 1] Cast Assassination Widget
  (cast `/Game/ThirdPerson/Blueprints/BP_ThirdPersonCharacter` OtherActor)
  (`SceneComponent.SetVisibility` (`self.AssasinateWidget`) true false))

(event `self.AssassinationSph.OnComponentEndOverlap`
  (params (OverlappedComponent :type "PrimitiveComponent Object Reference") (OtherActor :type "Actor Object Reference") (OtherComp :type "PrimitiveComponent Object Reference") (OtherBodyIndex :type Integer))
  ;[1 1 1] Cast Assassination Widget
  (cast `/Game/ThirdPerson/Blueprints/BP_ThirdPersonCharacter` OtherActor)
  (`SceneComponent.SetVisibility` (`self.AssasinateWidget`) false false))

(fn `StealthBackAssassination`
  (returns (REF_loc :type "Vector Structure") (AssasinRot :type "Rotator Structure"))
  (`self.PlayAnimMontage` "/Game/Characters/RPG_Character/Animation/Assassination/KnifeVic.KnifeVic")
  (`self.Ragdoll`)
  (`SceneComponent.SetVisibility` (`self.AssasinateWidget`) false false)
  (return (`SceneComponent.K2_GetComponentLocation` (`self.AssasinREF`)) (`self.K2_GetActorRotation`)))

(fn `UserConstructionScript`)