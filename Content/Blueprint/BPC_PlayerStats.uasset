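; Player stats component that tracks current and max health and stamina for BP_ThirdPersonCharacter.
; A tick after BeginPlay, it caches the owning character and initializes its HUD widget bars and health text.
; Increase functions raise maximums or add to current values capped at max, while decrease functions return true once the stat is depleted.
; Every stat change directly pushes the new percentage, plus the health value, to the HUD.
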(event `self.ReceiveBeginPlay`
  (bind _hud_widget (`/Game/ThirdPerson/Blueprints/BP_ThirdPersonCharacter.HUD Widget` (`self.PlayerCharacterBP`)))
  (`KismetSystemLibrary.DelayUntilNextTick`)
  (bind _asbp_third_person_character (cast `/Game/ThirdPerson/Blueprints/BP_ThirdPersonCharacter` (`self.GetOwner`)))
  (set `self.PlayerCharacterBP` _asbp_third_person_character)
  (`ProgressBar.SetPercent` (`/Game/UI/WB_HUD.StaminaBar` _hud_widget) (/ (`self.CurrentStamina`) (`self.MaxStamina`)))
  (`ProgressBar.SetPercent` (`/Game/UI/WB_HUD.HealthBar` _hud_widget) (/ (`self.CurrentHealth`) (`self.MaxHealth`)))
  (set `TextBlock.Text` (`KismetTextLibrary.Conv_DoubleToText` (`self.CurrentHealth`) "HalfToEven") (`/Game/UI/WB_HUD.HealthValue` _hud_widget)))

(fn `DecreaseHealth`
  (params (Damage :type "Float (double-precision)"))
  (returns (IsPlayerDead :type Boolean))
  (bind _hud_widget (`/Game/ThirdPerson/Blueprints/BP_ThirdPersonCharacter.HUD Widget` (`self.PlayerCharacterBP`)))
  (if (not (<= (`self.CurrentHealth`) 0.0))
    (set `self.CurrentHealth` (- (`self.CurrentHealth`) Damage))
    (`ProgressBar.SetPercent` (`/Game/UI/WB_HUD.HealthBar` _hud_widget) (/ (`self.CurrentHealth`) (`self.MaxHealth`)))
    (set `TextBlock.Text` (`KismetTextLibrary.Conv_DoubleToText` (`self.CurrentHealth`) "HalfToEven") (`/Game/UI/WB_HUD.HealthValue` _hud_widget))
    (if (<= (`self.CurrentHealth`) 0.0)
      _
      (else
        (return false))))
  (return true))

(fn `DecreaseStamina`
  (params (StaminaDec :type "Float (double-precision)"))
  (returns (noStaminaLeft :type Boolean))
  (if (not (<= (`self.CurrentStamina`) 0.0))
    (set `self.CurrentStamina` (- (`self.CurrentStamina`) StaminaDec))
    (`ProgressBar.SetPercent` (`/Game/UI/WB_HUD.StaminaBar` (`/Game/ThirdPerson/Blueprints/BP_ThirdPersonCharacter.HUD Widget` (`self.PlayerCharacterBP`))) (/ (`self.CurrentStamina`) (`self.MaxStamina`)))
    (if (<= (`self.CurrentStamina`) 0.0)
      _
      (else
        (return false))))
  (return true))

(fn `IncreaseHealth`
  (params (B :type "Float (double-precision)"))
  (bind _hud_widget (`/Game/ThirdPerson/Blueprints/BP_ThirdPersonCharacter.HUD Widget` (`self.PlayerCharacterBP`)))
  (set `self.CurrentHealth` (+ (`self.CurrentHealth`) B))
  (if (> (`self.CurrentHealth`) (`self.MaxHealth`))
    (set `self.CurrentHealth` (`self.MaxHealth`)))
  (`ProgressBar.SetPercent` (`/Game/UI/WB_HUD.HealthBar` _hud_widget) (/ (`self.CurrentHealth`) (`self.MaxHealth`)))
  (set `TextBlock.Text` (`KismetTextLibrary.Conv_DoubleToText` (`self.CurrentHealth`) "HalfToEven") (`/Game/UI/WB_HUD.HealthValue` _hud_widget)))

(fn `IncreaseMaxHealth`
  (params (MaxHealthInc :type "Float (double-precision)"))
  (bind _hud_widget (`/Game/ThirdPerson/Blueprints/BP_ThirdPersonCharacter.HUD Widget` (`self.PlayerCharacterBP`)))
  (set `self.MaxHealth` (+ (`self.MaxHealth`) MaxHealthInc))
  (`ProgressBar.SetPercent` (`/Game/UI/WB_HUD.HealthBar` _hud_widget) (/ (`self.CurrentHealth`) (`self.MaxHealth`)))
  (set `TextBlock.Text` (`KismetTextLibrary.Conv_DoubleToText` (`self.CurrentHealth`) "HalfToEven") (`/Game/UI/WB_HUD.HealthValue` _hud_widget)))

(fn `IncreaseStamina`
  (params (B :type "Float (double-precision)"))
  (set `self.CurrentStamina` (+ (`self.CurrentStamina`) B))
  (if (> (`self.CurrentStamina`) (`self.MaxStamina`))
    (set `self.CurrentStamina` (`self.MaxStamina`)))
  (`ProgressBar.SetPercent` (`/Game/UI/WB_HUD.StaminaBar` (`/Game/ThirdPerson/Blueprints/BP_ThirdPersonCharacter.HUD Widget` (`self.PlayerCharacterBP`))) (/ (`self.CurrentStamina`) (`self.MaxStamina`))))

(fn `InreaseMaxStamina`
  (params (MaxStaminaInc :type "Float (double-precision)"))
  (set `self.MaxStamina` (+ (`self.MaxStamina`) MaxStaminaInc))
  (`ProgressBar.SetPercent` (`/Game/UI/WB_HUD.StaminaBar` (`/Game/ThirdPerson/Blueprints/BP_ThirdPersonCharacter.HUD Widget` (`self.PlayerCharacterBP`))) (/ (`self.CurrentStamina`) (`self.MaxStamina`))))